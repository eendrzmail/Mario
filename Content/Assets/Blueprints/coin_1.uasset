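; Coin actor that swaps the material on its Box component when another actor overlaps it.
; BeginPlay resets a local coin counter with a maximum of one, and each overlap increments it up to that cap.
; Reaching the cap, or overlapping again afterwards, applies MaterialSwitch to the first material slot.
; The overlap does not filter the other actor, and the coin is never destroyed.
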(event Collision|EventActorBeginOverlap
  (params (OtherActor :type Actor%20Object%20Reference))
  (if (< (Variables|Default|GetCoins) (Variables|Default|GetMax_coins))
    (Variables|Default|SetCoins (+ (Variables|Default|GetCoins) 1))
    (if (== (Variables|Default|GetMax_coins) (Variables|Default|GetCoins))
      (Rendering|Material|SetMaterial (Variables|Default|GetBox) 0 (Variables|Default|GetMaterial_switch)))
    (else
      (Rendering|Material|SetMaterial (Variables|Default|GetBox) 0 (Variables|Default|GetMaterial_switch)))))

(event EventBeginPlay
  (Variables|Default|SetCoins 0)
  (Variables|Default|SetMax_coins 1))

(fn ConstructionScript)