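; Destructible brick actor for a side-scroller that shatters when any actor overlaps it.
; On overlap it disables collision on its CubeDM mesh, applies heavy damage with an upward impulse and switches physics simulation off.
; After short delays it makes the player's SideScrollerCharacter capsule ignore it when moving, then destroys itself and prints a debug message.
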(event EventBeginPlay)

(event Collision|EventActorBeginOverlap
  (params (OtherActor :type Actor%20Object%20Reference))
  (bind _cube_dm (Variables|Default|GetCube_DM))
  (Collision|SetCollisionEnabled _cube_dm "NoCollision")
  (Class|DestructibleComponent|ApplyDamage _cube_dm 5e+02 (Transformation|GetWorldLocation _cube_dm) (Math|Vector|MakeVector 0.0 0.0 5e+02) 6e+03)
  (Physics|SetSimulatePhysics (Variables|Default|GetCube_DM) false)
  (Utilities|FlowControl|Delay 0.1)
  (bind _asside_scroller_character (Utilities|Casting|CastToSideScrollerCharacter (Game|Player|GetPlayerPawn 0)))
  (Collision|IgnoreActorwhenMoving (Variables|/Script/Engine.Character|GetCapsuleComponent _asside_scroller_character) self true)
  (Utilities|FlowControl|Delay 5.0)
  (Actor|DestroyActor)
  (Development|PrintString "zniknieto"))

(event EventTick
  (params (DeltaSeconds :type Float%20%28single-precision%29)))

(fn ConstructionScript)